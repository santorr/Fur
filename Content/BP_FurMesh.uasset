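; Actor that renders shell-based fur over its static mesh, built in the construction script.
; CreateShells copies that mesh into the instanced Fur component, sets cull distances and adds instances based on fur length divided by interval.
; All shells share one M_Fur dynamic material carrying the look parameters, with each shell's index passed as per-instance custom data.
; SetMID, an alternative per-shell material builder, is never called here.
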(fn `CreateInstanceMaterial`
  (returns (ReturnValue :type "MaterialInstanceDynamic Object Reference"))
  (bind _returnvalue (`KismetMaterialLibrary.CreateDynamicMaterialInstance` "/Fur/M_Fur.M_Fur"))
  (`MaterialInstanceDynamic.SetScalarParameterValue` _returnvalue "Density" (`KismetMathLibrary.Conv_IntToDouble` (`self.Density`)))
  (`MaterialInstanceDynamic.SetScalarParameterValue` _returnvalue "Shell count" (`KismetMathLibrary.Conv_IntToDouble` 0))
  (`MaterialInstanceDynamic.SetScalarParameterValue` _returnvalue "Shell length" (`self.Length`))
  (`MaterialInstanceDynamic.SetScalarParameterValue` _returnvalue "Interval" (`self.Interval`))
  (`MaterialInstanceDynamic.SetScalarParameterValue` _returnvalue "Ambient occlusion attenuation" (`self.AmbientOcclusionAttenuation`))
  (`MaterialInstanceDynamic.SetScalarParameterValue` _returnvalue "Ambient occlusion bias" (`self.AmbientOcclusionBias`))
  (`MaterialInstanceDynamic.SetTextureParameterValue` _returnvalue "Color" (`self.Color`))
  (`MaterialInstanceDynamic.SetVectorParameterValue` _returnvalue "Teint" (`self.Teint`))
  (`MaterialInstanceDynamic.SetScalarParameterValue` _returnvalue "Color variation" (`self.ColorVariation`))
  (`MaterialInstanceDynamic.SetScalarParameterValue` _returnvalue "Normal intensity" (`self.NormalIntensity`))
  (`MaterialInstanceDynamic.SetTextureParameterValue` _returnvalue "Mask" (`self.Mask`))
  (return _returnvalue))

(fn `CreateShells`
  (bind _fur (`self.Fur`))
  (bind _cullingdistance (`self.CullingDistance`))
  (`InstancedStaticMeshComponent.SetCullDistances` _fur _cullingdistance _cullingdistance)
  (`StaticMeshComponent.SetStaticMesh` _fur (`StaticMeshComponent.StaticMesh` (`self.StaticMeshComponent`)))
  (bind _returnvalue (`self.CreateInstanceMaterial`))
  (`PrimitiveComponent.SetMaterial` _fur 0 _returnvalue)
  (for _index (range (+ (`KismetMathLibrary.Round` (/ (`self.Length`) (`self.Interval`))) 1))
    (`InstancedStaticMeshComponent.AddInstance` _fur (`KismetMathLibrary.MakeTransform` (0.0 0.0 0.0)) false)
    (`InstancedStaticMeshComponent.SetCustomDataValue` _fur _index 0 (+ (`KismetMathLibrary.Conv_IntToDouble` _index) 0.0001) false))
  (return))

(fn `SetMID`
  (params (index :type Integer))
  (returns (ReturnValue :type "MaterialInstanceDynamic Object Reference"))
  (locals (local_mid :type "MaterialInstanceDynamic Object Reference"))
  (`|ExecutionSequence`
    (:`then_0`
      (bind _returnvalue (`KismetMaterialLibrary.CreateDynamicMaterialInstance` "/Fur/M_Fur.M_Fur"))
      (set `local.local_mid` _returnvalue)
      (`MaterialInstanceDynamic.SetScalarParameterValue` (`local.local_mid`) "Density" (`KismetMathLibrary.Conv_IntToDouble` (`self.Density`)))
      (`MaterialInstanceDynamic.SetScalarParameterValue` (`local.local_mid`) "Shell index" (`KismetMathLibrary.Conv_IntToDouble` (`local.index`)))
      (`MaterialInstanceDynamic.SetScalarParameterValue` (`local.local_mid`) "Shell count" (`KismetMathLibrary.Conv_IntToDouble` 0))
      (`MaterialInstanceDynamic.SetScalarParameterValue` (`local.local_mid`) "Shell length" (`self.Length`))
      (`MaterialInstanceDynamic.SetScalarParameterValue` (`local.local_mid`) "Ambient occlusion attenuation" (`self.AmbientOcclusionAttenuation`))
      (`MaterialInstanceDynamic.SetScalarParameterValue` (`local.local_mid`) "Ambient occlusion bias" (`self.AmbientOcclusionBias`))
      (`MaterialInstanceDynamic.SetTextureParameterValue` (`local.local_mid`) "Color" (`self.Color`))
      (`MaterialInstanceDynamic.SetVectorParameterValue` (`local.local_mid`) "Teint" (`self.Teint`))
      (`MaterialInstanceDynamic.SetTextureParameterValue` (`local.local_mid`) "Mask" (`self.Mask`)))
    (:`then_1`
      (return (`local.local_mid`)))))

(fn `UserConstructionScript`
  (`self.CreateShells`))